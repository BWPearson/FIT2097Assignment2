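; FuseHolder is an interactable fuse socket that unlocks a linked Door when the player inserts a fuse.
; Overlapping its Box enables input on the actor from player controller 0, and leaving disables it.
; Pressing E reads HasFuse on the FirstPersonCharacter; if true, it shows the HiddenFuse component, clears that flag and sets the Door's IsLocked to false.
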(event `self.Box.OnComponentBeginOverlap`
  (params (OverlappedComponent :type "PrimitiveComponent Object Reference") (OtherActor :type "Actor Object Reference") (OtherComp :type "PrimitiveComponent Object Reference") (OtherBodyIndex :type Integer) (bFromSweep :type Boolean) (SweepResult :type "HitResult Structure (by ref)"))
  (`self.EnableInput` (`GameplayStatics.GetPlayerController` 0)))

(event `Key|E`
  (params (Key :type "Key Structure"))
  (:`Pressed`
    (bind _asfirst_person_character (cast `/Game/FirstPersonBP/Blueprints/FirstPersonCharacter` (`GameplayStatics.GetPlayerCharacter` 0))
      (:`then`
        _)
      (:`CastFailed`
        _))
    (bind _hasfuse (`/Game/FirstPersonBP/Blueprints/FirstPersonCharacter.HasFuse` _asfirst_person_character))
    (if _hasfuse
      (`SceneComponent.SetVisibility` (`self.HiddenFuse`) _hasfuse false)
      (set `/Game/FirstPersonBP/Blueprints/FirstPersonCharacter.HasFuse` false _asfirst_person_character)
      (set `/Game/StarterContent/Blueprints/BP_Doorhinge.IsLocked` false (`self.Door`)))))

(event `self.Box.OnComponentEndOverlap`
  (params (OverlappedComponent :type "PrimitiveComponent Object Reference") (OtherActor :type "Actor Object Reference") (OtherComp :type "PrimitiveComponent Object Reference") (OtherBodyIndex :type Integer))
  (`self.DisableInput` (`GameplayStatics.GetPlayerController` 0)))

(fn `UserConstructionScript`)