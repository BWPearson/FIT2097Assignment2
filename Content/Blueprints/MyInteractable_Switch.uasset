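; Interactable switch that slides its lever and locks or unlocks a referenced Door.
; Each Interact prints a debug message, flips IsOn, and plays the timeline when switching off or reverses it when switching on.
; Timeline updates lerp the Switch's relative location between lever start and end positions with sweep, and set the Door's IsLocked to match IsOn.
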(event `self.Interact`
  (bind _door (`self.Door`))
  (`KismetSystemLibrary.PrintString` "SWITCH IS ACTIVATED")
  (if (`self.IsOn`)
    (set `self.IsOn` false)
    (bind (_direction _switchslide) (`Timeline|Timeline_0` :!label _label)
      (:`Update`
        (`SceneComponent.K2_SetRelativeLocation` (`self.Switch`) (`KismetMathLibrary.VLerp` (`self.LeverStartPos`) (`self.LeverEndPos`) _switchslide) true false)
        (if (`self.IsOn`)
          (set `Door.IsLocked` true _door)
          (else
            (set `Door.IsLocked` false _door)))))
    (else
      (set `self.IsOn` true)
      (goto _label :!via `Reverse`))))

(fn `UserConstructionScript`)