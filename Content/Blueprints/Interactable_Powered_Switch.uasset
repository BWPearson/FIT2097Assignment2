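; Interactable lever switch with replicated movement that toggles a linked MyDoor open or closed.
; Each Interact flips IsOn and plays or reverses a timeline that slides the Switch component between start and end positions.
; On each timeline update, it casts Door to MyDoor and sets DoorIsOpen to the inverse of IsOn.
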(event `self.ReceiveBeginPlay`
  (`self.SetReplicateMovement` true)
  (`ActorComponent.SetIsReplicated` (`self.Switch`) true))

(event `self.Interact`
  (`KismetSystemLibrary.PrintString` "SWITCH IS ACTIVATED")
  (if (`self.IsOn`)
    (set `self.IsOn` false)
    (bind (_direction _switchslide) (`Timeline|Timeline_0` :!label _label)
      (:`Update`
        (`SceneComponent.K2_SetRelativeLocation` (`self.Switch`) (`KismetMathLibrary.VLerp` (`self.LeverStartPos`) (`self.LeverEndPos`) _switchslide) true false)
        (bind _asmy_door (cast `/Game/Blueprints/MyDoor` (`self.Door`)))
        (if (`self.IsOn`)
          (set `/Game/Blueprints/MyDoor.bDoorIsOpen` false _asmy_door)
          (else
            (set `/Game/Blueprints/MyDoor.bDoorIsOpen` true _asmy_door)))))
    (else
      (set `self.IsOn` true)
      (goto _label :!via `Reverse`))))

(fn `UserConstructionScript`)